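; DefaultPawnBP is a player pawn with six-degree-of-freedom, physics-driven movement.
; Pitch, yaw and roll axis inputs add angular velocity to the CollisionComponent, rotated from local axes by the actor's rotation.
; Forward and strafe inputs add linear velocity along the actor's forward, right and up vectors.
; Each input accumulates on the current velocity, scaled by speed variables but not by delta time.
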(event EventBeginPlay)

(event Collision|EventActorBeginOverlap
  (params (OtherActor :type Actor%20Object%20Reference)))

(event EventTick
  (params (DeltaSeconds :type Float%20%28single-precision%29)))

(event Input|AxisEvents|InputAxisForward
  (params (AxisValue :type Float%20%28single-precision%29))
  (Physics|SetPhysicsLinearVelocity (Variables|Default|GetCollisionComponent) (* (Math|Vector|GetForwardVector (Transformation|GetActorRotation)) (* AxisValue (Variables|Default|GetMoveSpeed))) true "None"))

(event Input|AxisEvents|InputAxisViewYaw
  (params (AxisValue :type Float%20%28single-precision%29))
  (Class|PrimitiveComponent|SetPhysicsAngularVelocityinDegrees (Variables|Default|GetCollisionComponent) (Math|Vector|RotateVector (Math|Vector|MakeVector 0.0 0.0 (* AxisValue (Variables|Default|GetYawSpeed))) (Transformation|GetActorRotation)) true "None"))

(event Input|AxisEvents|InputAxisStrafeRight
  (params (AxisValue :type Float%20%28single-precision%29))
  (Physics|SetPhysicsLinearVelocity (Variables|Default|GetCollisionComponent) (* (Math|Vector|GetRightVector (Transformation|GetActorRotation)) (* AxisValue (Variables|Default|GetMoveSpeed))) true "None"))

(event Input|AxisEvents|InputAxisViewPitch
  (params (AxisValue :type Float%20%28single-precision%29))
  (Class|PrimitiveComponent|SetPhysicsAngularVelocityinDegrees (Variables|Default|GetCollisionComponent) (Math|Vector|RotateVector (Math|Vector|MakeVector 0.0 (* AxisValue (Variables|Default|GetPitchSpeed)) 0.0) (Transformation|GetActorRotation)) true "None"))

(event Input|AxisEvents|InputAxisRollLeft
  (params (AxisValue :type Float%20%28single-precision%29))
  (Class|PrimitiveComponent|SetPhysicsAngularVelocityinDegrees (Variables|Default|GetCollisionComponent) (Math|Vector|RotateVector (Math|Vector|MakeVector (* AxisValue (Variables|Default|GetRollSpeed)) 0.0 0.0) (Transformation|GetActorRotation)) true "None"))

(event Input|AxisEvents|InputAxisStrafeUp
  (params (AxisValue :type Float%20%28single-precision%29))
  (Physics|SetPhysicsLinearVelocity (Variables|Default|GetCollisionComponent) (* (Math|Vector|GetUpVector (Transformation|GetActorRotation)) (* AxisValue (Variables|Default|GetMoveSpeed))) true "None"))

(fn ConstructionScript)