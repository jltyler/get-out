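; Door actor that swings open and shut around its yaw when its DoorRotator component fires open or close events.
; The construction script stores the actor's starting rotation on DoorRotator as the closed pose.
; OpenTimeline drives SetRotationFromAlpha, lerping yaw from that pose by the component's OpenAngle.
; Closing reverses the same timeline at a faster play rate, so the door shuts quicker than it opens.
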(event OnOpenDoor(DoorRotator)
  (Components|Timeline|SetPlayRate (Variables|Default|GetOpenTimeline) 1.0)
  (bind _rotationalpha (Timeline|OpenTimeline Play)
    (:Update
      (CallFunction|SetRotationfromAlpha _rotationalpha))))

(event OnCloseDoor(DoorRotator)
  (Components|Timeline|SetPlayRate (Variables|Default|GetOpenTimeline) 3.0)
  (bind _rotationalpha (Timeline|OpenTimeline Reverse)
    (:Update
      (CallFunction|SetRotationfromAlpha _rotationalpha))))

(event EventBeginPlay)

(event Collision|EventActorBeginOverlap
  (params (OtherActor :type Actor%20Object%20Reference)))

(event EventTick
  (params (DeltaSeconds :type Float%20%28single-precision%29)))

(fn ConstructionScript
  (Variables|/Script/GetOUT.DoorRotator|SetOriginalRotation (Variables|Default|GetDoorRotator) (Transformation|GetActorRotation)))

(fn SetRotationfromAlpha
  (params (Alpha :type Float%20%28single-precision%29))
  (bind _doorrotator (Variables|Default|GetDoorRotator))
  (bind _originalrotation (Variables|/Script/GetOUT.DoorRotator|GetOriginalRotation _doorrotator))
  (bind (_roll _pitch _yaw) (Math|Rotator|BreakRotator _originalrotation))
  (bind _returnvalue (Transformation|SetActorRotation (Math|Rotator|MakeRotator _roll _pitch (Math|Float|Lerp _yaw (+ _yaw (Variables|/Script/GetOUT.DoorRotator|GetOpenAngle _doorrotator)) Alpha))))
  (return _returnvalue))