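; DoorCircleCornerBP is a door actor that swings four door pieces open and shut in response to its DoorRotator's open and close events.
; One timeline, played forward or reversed at separate open and close rates, lerps the pitch of four scene components from zero to the rotator's OpenAngle.
; A blocking box loses collision as soon as opening starts and regains it as soon as closing starts.
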(event OnOpenDoor(DoorRotator)
  (Collision|SetCollisionEnabled (Variables|Default|GetBlockingBox) "NoCollision")
  (Components|Timeline|SetPlayRate (Variables|Default|GetDoorTimeline) (Variables|DoorOptions|GetOpenRate))
  (bind _newtrack_0 (Timeline|DoorTimeline Play)
    (:Update
      (Transformation|SetRelativeRotation (Variables|Default|GetDoorScene2) (Math|Rotator|MakeRotator 0.0 (Math|Float|Lerp 0.0 (Variables|/Script/GetOUT.DoorRotator|GetOpenAngle (Variables|Default|GetDoorRotator)) _newtrack_0) 0.0) false false))))

(event OnCloseDoor(DoorRotator)
  (Collision|SetCollisionEnabled (Variables|Default|GetBlockingBox) "QueryAndPhysics")
  (Components|Timeline|SetPlayRate (Variables|Default|GetDoorTimeline) (Variables|DoorOptions|GetCloseRate))
  (bind _newtrack_0 (Timeline|DoorTimeline Reverse)
    (:Update
      (Transformation|SetRelativeRotation (Variables|Default|GetDoorScene2) (Math|Rotator|MakeRotator 0.0 (Math|Float|Lerp 0.0 (Variables|/Script/GetOUT.DoorRotator|GetOpenAngle (Variables|Default|GetDoorRotator)) _newtrack_0) 0.0) false false))))

(event EventBeginPlay)

(event Collision|EventActorBeginOverlap
  (params (OtherActor :type Actor%20Object%20Reference)))

(event EventTick
  (params (DeltaSeconds :type Float%20%28single-precision%29)))

(fn ConstructionScript)